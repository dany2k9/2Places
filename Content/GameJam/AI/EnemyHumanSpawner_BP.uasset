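; EnemyHumanSpawner_BP spawns Enemy2 actors after random delays, starting on play or through ActivateSpawner2.
; It uses its own transform or the first SpawnPoint_BP with a matching ID, as random selection is unwired.
; With exactly one matching point, it only stores the location and the loop ends without spawning.
; Count limits the spawns before the spawner destroys itself, with -1 meaning endless.
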(event `self.ReceiveBeginPlay`
  (`|ExecutionSequence`
    (:`then_0`
      (if (`self.UseSpawnPoint`)
        (bind _outactors (`GameplayStatics.GetAllActorsOfClass` "/Game/GameJam/AI/SpawnPoint_BP.SpawnPoint_BP_C"))
        (for _array_element _outactors
          (if (`KismetStringLibrary.EqualEqual_StrStr` (`/Game/GameJam/AI/SpawnPoint_BP.SpawnPoint_ID` _array_element) (`self.SpawnPoint_ID`))
            (`KismetArrayLibrary.Array_AddUnique` (`self.SpawnPoints`) _array_element)))))
    (:`then_1`
      (if (`self.StartActive`)
        (`self.StartSpawning2`)))))

(event `StartSpawning2`
  (bind (_spawnlocation_location _spawnlocation_rotation) (`KismetMathLibrary.BreakTransform` (`self.SpawnLocation`)))
  (`KismetSystemLibrary.Delay` (`KismetMathLibrary.RandomFloatInRange` (`self.SpawnDelay_min`) (`self.SpawnDelay_max`)) :!label _label)
  (if (`self.UseSpawnPoint`)
    (if (== (`KismetArrayLibrary.Array_Length` (`self.SpawnPoints`)) 1)
      (set `self.SpawnLocation` (`self.GetTransform` (`|GetArrayItem` (`self.SpawnPoints`))))
      (else
        (set `self.SpawnLocation` (`self.GetTransform` (`|GetArrayItem` (`self.SpawnPoints`))))
        (`|SpawnActorFromClass` "/Game/GameJam/AI/Enemy2.Enemy2_C" (`KismetMathLibrary.MakeTransform` (+ _spawnlocation_location (0.0 0.0 3.0)) _spawnlocation_rotation) "Undefined" "OverrideRootScale" null null :!label _label_2)
        (if (== (`self.Count`) -1)
          (goto _label)
          (else
            (set `self.Count` (- (`self.Count`) 1))
            (if (> (`self.Count`) 0)
              (goto _label)
              (else
                (`KismetSystemLibrary.Delay` 0.5)
                (`self.K2_DestroyActor`)))))))
    (else
      (set `self.SpawnLocation` (`self.GetTransform`))
      (goto _label_2))))

(event `ActivateSpawner2`
  (`self.StartSpawning2`))

(fn `UserConstructionScript`)